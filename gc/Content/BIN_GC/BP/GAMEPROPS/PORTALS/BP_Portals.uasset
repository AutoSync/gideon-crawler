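; BP_Portals is a teleport portal that moves the 2D player to a linked exit portal.
; When its trigger component is overlapped, it fetches player character 0 as BP_Player2D_GC and, if that player is moving, teleports it to the TriggerArrow transform of PortalOutput.
; The overlapping actor is never checked, and a portal without a valid output prints a missing-exit message.
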(event `self.Trigger_portal.OnComponentBeginOverlap`
  (params (OverlappedComponent :type "PrimitiveComponent Object Reference") (OtherActor :type "Actor Object Reference") (OtherComp :type "PrimitiveComponent Object Reference") (OtherBodyIndex :type Integer) (bFromSweep :type Boolean) (SweepResult :type "HitResult Structure (by ref)"))
  (`/Engine/EditorBlueprintResources/StandardMacros.IsValid` (`self.Portal Output`)
    (:`Is Valid`
      (bind _asgc_player_2d (cast `/Game/BIN_GC/BP/PLAYER/MASTER/BP_Player2D_GC` (`GameplayStatics.GetPlayerCharacter` 0)))
      (`/Engine/EditorBlueprintResources/StandardMacros.IsValid` _asgc_player_2d
        (:`Is Valid`
          (if (`/Game/BIN_GC/BP/PLAYER/MASTER/BP_Player2D_GC.InMoving?` _asgc_player_2d)
            (`self.K2_SetActorTransform` _asgc_player_2d (`SceneComponent.K2_GetComponentToWorld` (`/Game/BIN_GC/BP/GAMEPROPS/PORTALS/BP_Portals.Trigger_Arrow` (`self.Portal Output`))) false true)))))
    (:`Is Not Valid`
      (`KismetSystemLibrary.PrintText` "Sem Saida Definida"))))

(fn `UserConstructionScript`)