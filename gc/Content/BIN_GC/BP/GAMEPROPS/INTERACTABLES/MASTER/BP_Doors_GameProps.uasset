(event `self.ReceiveBeginPlay`
  (`self.Build`))

(event `OpenDoor`
  (bind _sprite_open (`self.Sprite Open`))
  (bind _box_collision (`self.Box_Collision`))
  (bind _box_trigger (`self.Box_Trigger`))
  ; Eventos de Abrir e Fechar Porta
  (`PaperSpriteComponent.SetSprite` (`self.LeftDoor_Sprite`) _sprite_open)
  (`PaperSpriteComponent.SetSprite` (`self.RightDoor_Sprite`) _sprite_open)
  (`PrimitiveComponent.SetCollisionEnabled` _box_collision "NoCollision")
  (`PrimitiveComponent.SetCollisionResponseToAllChannels` _box_collision "ECR_Ignore")
  (`PrimitiveComponent.SetCollisionEnabled` _box_trigger "NoCollision")
  (`PrimitiveComponent.SetCollisionResponseToAllChannels` _box_trigger "ECR_Ignore"))

(event `CloseDoor`
  (bind _sprite_closed (`self.Sprite Closed`))
  (bind _box_collision (`self.Box_Collision`))
  (bind _box_trigger (`self.Box_Trigger`))
  ; Eventos de Abrir e Fechar Porta
  (`PaperSpriteComponent.SetSprite` (`self.LeftDoor_Sprite`) _sprite_closed)
  (`PaperSpriteComponent.SetSprite` (`self.RightDoor_Sprite`) _sprite_closed)
  (`PrimitiveComponent.SetCollisionEnabled` _box_collision "QueryAndPhysics")
  (`PrimitiveComponent.SetCollisionResponseToAllChannels` _box_collision "ECR_Block")
  (`PrimitiveComponent.SetCollisionEnabled` _box_trigger "QueryOnly")
  (`PrimitiveComponent.SetCollisionResponseToAllChannels` _box_trigger "ECR_Overlap"))

(event `Build`
  ; When loading the game or a save file, should the doors already opened in the level be loaded or not
  (if (`self.IsLocked?`)
    (set `self.Open?` false)
    (`self.CloseDoor` :!label _label)
    (elif (`self.Open?`)
      (`self.OpenDoor`)
      (else
        (goto _label)))))

(event `self.Box_Trigger.OnComponentBeginOverlap`
  (params (OverlappedComponent :type "PrimitiveComponent Object Reference") (OtherActor :type "Actor Object Reference") (OtherComp :type "PrimitiveComponent Object Reference") (OtherBodyIndex :type Integer) (bFromSweep :type Boolean) (SweepResult :type "HitResult Structure (by ref)"))
  ; Entrar na Colisão da Porta
  (bind _asbp_player_2d_gc (cast `/Game/BIN_GC/BP/PLAYER/MASTER/BP_Player2D_GC` (`GameplayStatics.GetPlayerPawn` 0)))
  (set `/Game/BIN_GC/BP/PLAYER/MASTER/BP_Player2D_GC.CurrentInteractable` self _asbp_player_2d_gc))

(event `TryUnlock`
  (params (Interactor :type "Actor Object Reference"))
  (`/Engine/EditorBlueprintResources/StandardMacros.IsValid` Interactor
    (:`Is Not Valid`
      (`self.CheckItemInventory`))))

(event `self.Box_Trigger.OnComponentEndOverlap`
  (params (OverlappedComponent :type "PrimitiveComponent Object Reference") (OtherActor :type "Actor Object Reference") (OtherComp :type "PrimitiveComponent Object Reference") (OtherBodyIndex :type Integer))
  ; Sair da Colisão da Porta
  (bind _asbp_player_2d_gc (cast `/Game/BIN_GC/BP/PLAYER/MASTER/BP_Player2D_GC` (`GameplayStatics.GetPlayerPawn` 0)))
  (if (== (`/Game/BIN_GC/BP/PLAYER/MASTER/BP_Player2D_GC.CurrentInteractable` _asbp_player_2d_gc) self)
    (set `/Game/BIN_GC/BP/PLAYER/MASTER/BP_Player2D_GC.CurrentInteractable` null _asbp_player_2d_gc)))

(event `CheckItemInventory`
  ; Open Ivenotry -> Compare key -> Access Allow || Close inventory
  (bind _asbp_player_2d_gc (cast `/Game/BIN_GC/BP/PLAYER/MASTER/BP_Player2D_GC` (`GameplayStatics.GetPlayerCharacter` 0)))
  (`/Game/BIN_GC/BP/PLAYER/MASTER/BP_Player2D_GC.Evt_OpenInventoryForTarget` _asbp_player_2d_gc self true))

(event `/Game/BIN_GC/BP/GAMEPROPS/INTERACTABLES/INTERFACES/BPI_Interactable_GC.Interact`
  (params (Interactor :type "Actor Object Reference"))
  ; Interact With Door
  (if (`self.Open?`)
    (`self.OpenDoor`)
    (elif (`self.IsLocked?`)
      (`self.TryUnlock` null)
      (else
        (`self.CloseDoor`)))))

(fn `TryReceiveItem`
  (params (ItemData :type "/Game/BIN_GC/BP/GAMEPROPS/INTERACTABLES/DATAASSET/DA_InventoryItem Object Reference"))
  (returns (Result :type "/Game/BIN_GC/BP/GAMEPROPS/INTERACTABLES/ENUMS/E_ItemUseResult Enum") (ConsumeItemUse :type Boolean) (Message :type Text))
  (if (`self.IsLocked?`)
    (if (and (`|EnumEquality` (`/Game/BIN_GC/BP/GAMEPROPS/INTERACTABLES/DATAASSET/DA_InventoryItem.ItemType` ItemData) (`self.RequiredItemType`)) (== (`/Game/BIN_GC/BP/GAMEPROPS/INTERACTABLES/DATAASSET/DA_InventoryItem.ItemCode` ItemData) (`self.RequiredItemCode`)))
      (set `self.IsLocked?` false)
      (`self.OpenDoor`)
      (return "NewEnumerator3" true "item.result.sucessDoor")
      (else
        (return "NewEnumerator5" false "item.result.wrongitem")))
    (else
      (return "NewEnumerator6" false "item.result.alreadyUnlocked"))))

(fn `UserConstructionScript`
  (`self.Build`))