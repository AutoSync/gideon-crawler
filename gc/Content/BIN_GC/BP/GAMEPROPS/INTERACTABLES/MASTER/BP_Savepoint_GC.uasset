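; BP_Savepoint_GC is an interactable savepoint prop whose Interact event is empty, so no save logic runs here.
; Its Trigger component's begin overlap registers the savepoint as CurrentInteractable on player character 0, cast to BP_Player2D_GC.
; End overlap clears that reference only if it still points to this savepoint.
; Neither overlap event checks which actor caused it.
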(event `self.Trigger.OnComponentBeginOverlap`
  (params (OverlappedComponent :type "PrimitiveComponent Object Reference") (OtherActor :type "Actor Object Reference") (OtherComp :type "PrimitiveComponent Object Reference") (OtherBodyIndex :type Integer) (bFromSweep :type Boolean) (SweepResult :type "HitResult Structure (by ref)"))
  (bind _asgc_player_2d (cast `/Game/BIN_GC/BP/PLAYER/MASTER/BP_Player2D_GC` (`GameplayStatics.GetPlayerCharacter` 0)))
  (set `/Game/BIN_GC/BP/PLAYER/MASTER/BP_Player2D_GC.CurrentInteractable` self _asgc_player_2d))

(event `self.Trigger.OnComponentEndOverlap`
  (params (OverlappedComponent :type "PrimitiveComponent Object Reference") (OtherActor :type "Actor Object Reference") (OtherComp :type "PrimitiveComponent Object Reference") (OtherBodyIndex :type Integer))
  (bind _asgc_player_2d (cast `/Game/BIN_GC/BP/PLAYER/MASTER/BP_Player2D_GC` (`GameplayStatics.GetPlayerCharacter` 0)))
  (if (== (`/Game/BIN_GC/BP/PLAYER/MASTER/BP_Player2D_GC.CurrentInteractable` _asgc_player_2d) self)
    (set `/Game/BIN_GC/BP/PLAYER/MASTER/BP_Player2D_GC.CurrentInteractable` null _asgc_player_2d)))

(event `/Game/BIN_GC/BP/GAMEPROPS/INTERACTABLES/INTERFACES/BPI_Interactable_GC.Interact`
  (params (InteractActor :type "Actor Object Reference")))

(fn `UserConstructionScript`)