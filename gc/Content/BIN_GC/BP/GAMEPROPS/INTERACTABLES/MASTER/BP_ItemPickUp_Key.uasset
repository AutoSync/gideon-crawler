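; BP_ItemPickUp_Key is an interactable key pickup that the player collects into their inventory.
; On Interact it casts the player character to GC_Player2D and adds its TypeData to InventoryItems.
; A successful add destroys the actor; otherwise it prints an inventory-full message, noted as a placeholder for UI.
; The trigger's begin overlap only performs the player cast and does nothing further.
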(event `self.Trigger.OnComponentBeginOverlap`
  (params (OverlappedComponent :type "PrimitiveComponent Object Reference") (OtherActor :type "Actor Object Reference") (OtherComp :type "PrimitiveComponent Object Reference") (OtherBodyIndex :type Integer) (bFromSweep :type Boolean) (SweepResult :type "HitResult Structure (by ref)"))
  (cast `/Game/BIN_GC/BP/PLAYER/MASTER/GC_Player2D` (`GameplayStatics.GetPlayerCharacter` 0)))

(event `self.Trigger.OnComponentEndOverlap`
  (params (OverlappedComponent :type "PrimitiveComponent Object Reference") (OtherActor :type "Actor Object Reference") (OtherComp :type "PrimitiveComponent Object Reference") (OtherBodyIndex :type Integer)))

(event `/Game/BIN_GC/BP/GAMEPROPS/INTERACTABLES/INTERFACES/BPI_Interactable_GC.Interact`
  (params (InteractActor :type "Actor Object Reference"))
  ; Add item to Inventory
  (bind _asgc_player_2d (cast `/Game/BIN_GC/BP/PLAYER/MASTER/GC_Player2D` (`GameplayStatics.GetPlayerCharacter` 0)))
  (bind _success (`/Game/BIN_GC/BP/PLAYER/MASTER/BP_InventoryComponent.AddItem` (`/Game/BIN_GC/BP/PLAYER/MASTER/GC_Player2D.InventoryItems` _asgc_player_2d) (`self.TypeData`)))
  (if _success
    (`self.K2_DestroyActor`)
    (else
      ;; Substituir por menssagem em via UI
      (`KismetSystemLibrary.PrintText` "Inventario Cheio"))))

(fn `UserConstructionScript`)