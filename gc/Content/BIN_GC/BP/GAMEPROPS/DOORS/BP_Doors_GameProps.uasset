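; A 2D door prop that the GC_Player2D pawn can interact with, registering itself as the player's CurrentInteractable while in its trigger box.
; Build, run from the construction script, and Interact use Open and IsLocked to swap both door sprites and toggle blocking collision, or check for an item.
; The lock check is a stub: CheckItem always returns true, and the result only sets CanOpen and prints a message.
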(event `self.ReceiveBeginPlay`)

(event `Build`
  ; When loading the game or a save file, should the doors already opened in the level be loaded or not
  (if (`self.IsLocked?`)
    (`self.CheckItemInventory`)
    (elif (`self.Open?`)
      (`self.OpenDoor`)
      (else
        (`self.CloseDoor`)))))

(event `OpenDoor`
  (bind _sprite_open (`self.Sprite Open`))
  (`PaperSpriteComponent.SetSprite` (`self.LeftDoor_Sprite`) _sprite_open)
  (`PaperSpriteComponent.SetSprite` (`self.RightDoor_Sprite`) _sprite_open)
  (`PrimitiveComponent.SetCollisionEnabled` (`self.Box_Collision`) "NoCollision"))

(event `CheckItemInventory`
  ; Open Ivenotry -> Compare key -> Access Allow || Close inventory
  (bind _isvaliditem_ (`self.CheckItem`))
  (bind _output_get (set `self.CanOpen?` _isvaliditem_))
  (if _output_get
    (`KismetSystemLibrary.PrintText` "Acesso Liberado")
    (else
      (`KismetSystemLibrary.PrintText` "Não funciona aqui"))))

(event `CloseDoor`
  (bind _sprite_closed (`self.Sprite Closed`))
  (`PaperSpriteComponent.SetSprite` (`self.LeftDoor_Sprite`) _sprite_closed)
  (`PaperSpriteComponent.SetSprite` (`self.RightDoor_Sprite`) _sprite_closed)
  (`PrimitiveComponent.SetCollisionEnabled` (`self.Box_Collision`) "QueryAndPhysics"))

(event `TryUnlock`
  (params (Interactor :type "Actor Object Reference"))
  (`/Engine/EditorBlueprintResources/StandardMacros.IsValid` Interactor
    (:`Is Not Valid`
      (`self.CheckItemInventory`))))

(event `self.Box_Trigger.OnComponentBeginOverlap`
  (params (OverlappedComponent :type "PrimitiveComponent Object Reference") (OtherActor :type "Actor Object Reference") (OtherComp :type "PrimitiveComponent Object Reference") (OtherBodyIndex :type Integer) (bFromSweep :type Boolean) (SweepResult :type "HitResult Structure (by ref)"))
  ; Entrar na Colisão da Porta
  (bind _asgc_player_2d (cast `/Game/BIN_GC/BP/PLAYER/MASTER/GC_Player2D` (`GameplayStatics.GetPlayerPawn` 0)))
  (set `/Game/BIN_GC/BP/PLAYER/MASTER/GC_Player2D.CurrentInteractable` self _asgc_player_2d)
  (`KismetSystemLibrary.PrintText` "Press to Interact with door"))

(event `self.Box_Trigger.OnComponentEndOverlap`
  (params (OverlappedComponent :type "PrimitiveComponent Object Reference") (OtherActor :type "Actor Object Reference") (OtherComp :type "PrimitiveComponent Object Reference") (OtherBodyIndex :type Integer))
  ; Sair da Colisão da Porta
  (bind _asgc_player_2d (cast `/Game/BIN_GC/BP/PLAYER/MASTER/GC_Player2D` (`GameplayStatics.GetPlayerPawn` 0)))
  (if (== (`/Game/BIN_GC/BP/PLAYER/MASTER/GC_Player2D.CurrentInteractable` _asgc_player_2d) self)
    (set `/Game/BIN_GC/BP/PLAYER/MASTER/GC_Player2D.CurrentInteractable` null _asgc_player_2d)))

(event `/Game/BIN_GC/BP/GAMEPROPS/INTERACTABLES/INTERFACES/BPI_Interactable_GC.Interact`
  (params (InteractActor :type "Actor Object Reference"))
  (if (`self.Open?`)
    (`self.CloseDoor`)
    (elif (`self.IsLocked?`)
      (`self.TryUnlock` null)
      (else
        (`self.OpenDoor`)))))

(fn `CheckItem`
  (returns (`IsValidItem?` :type Boolean))
  (return true))

(fn `UserConstructionScript`
  (`self.Build`))