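; Player inventory Blueprint that stores items in an array capped by an item limit.
; AddItem appends a new entry without stacking and reports failure when the inventory is full.
; TryUseItem finds the first in-stock match by type and code through HasItem, then passes its index to ConsumeItemByIndex.
; Consuming rewrites the entry with a decremented quantity, or removes it when the last unit is used.
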(fn `AddItem`
  (params (Item :type "/Game/BIN_GC/BP/GAMEPROPS/INTERACTABLES/STRUCT/SInventoryItem Structure"))
  (returns (Success :type Boolean))
  (bind _inventoryitems (`self.InventoryItems`))
  (if (== (`KismetArrayLibrary.Array_Length` _inventoryitems) (`self.Limit Items`))
    (return false)
    (else
      (`KismetArrayLibrary.Array_Add` _inventoryitems Item)
      (return true))))

(fn `ConsumeItemByIndex`
  (params (Index :type Integer))
  (returns (Success :type Boolean))
  (bind _inventoryitems (`self.InventoryItems`))
  (bind ((`Quantity_6_A3398DEB48D0123243C31E95099F5FE7` _quantity)) (break `/Game/BIN_GC/BP/GAMEPROPS/INTERACTABLES/STRUCT/SInventoryItem` (`|GetArrayItem` _inventoryitems Index)))
  (if (`KismetArrayLibrary.Array_IsValidIndex` _inventoryitems Index)
    (if (> _quantity 1)
      (`KismetArrayLibrary.Array_Set` _inventoryitems Index (make `/Game/BIN_GC/BP/GAMEPROPS/INTERACTABLES/STRUCT/SInventoryItem` :`Quantity` (- _quantity 1)))
      (return true)
      (elif (== _quantity 1)
        (`KismetArrayLibrary.Array_Remove` _inventoryitems Index)
        (return true)))
    (else
      (return false))))

(fn `HasItem`
  (params (RequitedItemType :type "/Game/BIN_GC/BP/GAMEPROPS/INTERACTABLES/ENUMS/EItemTypeGC Enum" :default "NewEnumerator0") (RequitedItemCode :type Name))
  (returns (Found :type Boolean) (ItemIndex :type Integer))
  (for (_array_element _array_index) (`self.InventoryItems`)
    (bind (_itemtype _itemcode _quantity) (break `/Game/BIN_GC/BP/GAMEPROPS/INTERACTABLES/STRUCT/SInventoryItem` _array_element))
    (if (and (`|EnumEquality` _itemtype RequitedItemType) (== _itemcode RequitedItemCode) (> _quantity 0))
      (return true _array_index)))
  (return false -1))

(fn `TryUseItem`
  (params (RequiredItemType :type "/Game/BIN_GC/BP/GAMEPROPS/INTERACTABLES/ENUMS/EItemTypeGC Enum" :default "NewEnumerator0") (RequiredItemCode :type Name))
  (returns (Success :type Boolean))
  (bind (_found _itemindex) (`self.HasItem` RequiredItemType RequiredItemCode))
  (if _found
    (bind _success (`self.ConsumeItemByIndex` _itemindex))
    (return _success)
    (else
      (return false))))

(fn `UserConstructionScript`)