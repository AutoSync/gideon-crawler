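; Player inventory component that stores items in an array capped at a maximum slot count.
; Items are looked up by type and code, then consumed by decrementing quantity or removing the entry.
; Contextual use passes the item to a target through BPI_ItemUseTarget, which returns a result, message key and whether to consume it.
; A separate function tracks limited uses, skipping items with infinite uses.
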(fn `AddItem`
  (params (Item :type "/Game/BIN_GC/BP/GAMEPROPS/INTERACTABLES/STRUCT/S_InventoryItem Structure"))
  (returns (Success :type Boolean))
  (bind _inventoryitems (`self.InventoryItems`))
  (bind _returnvalue (`KismetArrayLibrary.Array_Length` _inventoryitems))
  (if (== _returnvalue (`self.MaxSlotItems`))
    (return false)
    (else
      (`KismetArrayLibrary.Array_Add` _inventoryitems Item)
      (`KismetSystemLibrary.PrintText` (`|FormatText` "Item Adicionado Total de Items {items}" _returnvalue))
      (return true))))

(fn `ConsumeItemByIndex`
  (params (Index :type Integer))
  (returns (Success :type Boolean))
  (bind _inventoryitems (`self.InventoryItems`))
  (bind ((`Quantity_6_A3398DEB48D0123243C31E95099F5FE7` _quantity)) (break `/Game/BIN_GC/BP/GAMEPROPS/INTERACTABLES/STRUCT/S_InventoryItem` (`|GetArrayItem` _inventoryitems Index)))
  (if (`KismetArrayLibrary.Array_IsValidIndex` _inventoryitems Index)
    (if (> _quantity 1)
      (`KismetArrayLibrary.Array_Set` _inventoryitems Index (make `/Game/BIN_GC/BP/GAMEPROPS/INTERACTABLES/STRUCT/S_InventoryItem` :`Quantity` (- _quantity 1)))
      (return true)
      (elif (== _quantity 1)
        (`KismetArrayLibrary.Array_Remove` _inventoryitems Index)
        (return true)))
    (else
      (return false))))

(fn `ConsumeItemUse`
  (params (Index :type Integer))
  (bind _inventoryitems (`self.InventoryItems`))
  (bind ((`UsesRemain_23_8B29F7BE492704D2B547C8BCB866C626` _usesremain) (`InfinityUses_28_3264C86545264EBC95FD2893C8D54C7C` _infinityuses)) (break `/Game/BIN_GC/BP/GAMEPROPS/INTERACTABLES/STRUCT/S_InventoryItem` (`|GetArrayItem` (`self.InventoryItems`) Index)))
  (if _infinityuses
    _
    (elif (<= _usesremain 0)
      (`KismetArrayLibrary.Array_Remove` _inventoryitems Index)
      (else
        (`KismetArrayLibrary.Array_Set` _inventoryitems Index (make `/Game/BIN_GC/BP/GAMEPROPS/INTERACTABLES/STRUCT/S_InventoryItem` :`UsesRemain` (- _usesremain 1)))))))

(fn `HasItem`
  (params (RequitedItemType :type "/Game/BIN_GC/BP/GAMEPROPS/INTERACTABLES/ENUMS/E_ItemType Enum" :default "NewEnumerator0") (RequitedItemCode :type Name))
  (returns (Found :type Boolean) (ItemIndex :type Integer))
  (for (_array_element _array_index) (`self.InventoryItems`)
    (bind (_itemtype _itemcode _quantity) (break `/Game/BIN_GC/BP/GAMEPROPS/INTERACTABLES/STRUCT/S_InventoryItem` _array_element))
    (if (and (`|EnumEquality` _itemtype RequitedItemType) (== _itemcode RequitedItemCode) (> _quantity 0))
      (return true _array_index)))
  (return false -1))

(fn `TryUseItem`
  (params (RequiredItemType :type "/Game/BIN_GC/BP/GAMEPROPS/INTERACTABLES/ENUMS/E_ItemType Enum" :default "NewEnumerator0") (RequiredItemCode :type Name))
  (returns (Success :type Boolean))
  (bind (_found _itemindex) (`self.HasItem` RequiredItemType RequiredItemCode))
  (if _found
    (bind _success (`self.ConsumeItemByIndex` _itemindex))
    (return _success)
    (else
      (return false))))

(fn `TryUseItemAtIndex`
  (params (ItemIntex :type Integer) (UseContextTarget :type "Actor Object Reference"))
  (returns (Result :type "/Game/BIN_GC/BP/GAMEPROPS/INTERACTABLES/ENUMS/E_ItemUseResult Enum") (Message :type Text))
  (if (`KismetArrayLibrary.Array_IsValidIndex` (`self.InventoryItems`) ItemIntex)
    (`/Engine/EditorBlueprintResources/StandardMacros.IsValid` UseContextTarget
      (:`Is Valid`
        (if (`KismetSystemLibrary.DoesImplementInterface` UseContextTarget "/Game/BIN_GC/BP/GAMEPROPS/INTERACTABLES/INTERFACES/BPI_ItemUseTarget.BPI_ItemUseTarget_C")
          (bind (_result _consumeitemuse _message) (message `/Game/BIN_GC/BP/GAMEPROPS/INTERACTABLES/INTERFACES/BPI_ItemUseTarget.TryReceiveItem` UseContextTarget (`|GetArrayItem` (`self.InventoryItems`) ItemIntex)))
          (if (`|EnumEquality` _result "NewEnumerator3")
            (if _consumeitemuse
              (`self.ConsumeItemByIndex` ItemIntex)
              (else
                (return _result _message)))
            (else
              (return _result _message)))
          (else
            (return "NewEnumerator1" "item.result.CannotUseHere"))))
      (:`Is Not Valid`
        (return "NewEnumerator1" "item.result.CannotUseHere")))
    (else
      (return "NewEnumerator0" "item.result.InvalidItem"))))