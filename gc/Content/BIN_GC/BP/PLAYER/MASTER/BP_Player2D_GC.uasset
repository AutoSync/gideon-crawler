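; Player character for a 2D-sprite style game, handling movement, interaction, inventory and message dialogs.
; Enhanced Input moves the actor and records a dead-zoned facing direction for animation; leftward input currently maps to FrontSide, not LeftSide.
; Interact calls BPI_Interactable_GC on the current interactable.
; The inventory widget opens normally or for a target context, switching input mode and blocking movement; LoadData is an empty stub.
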(event `self.ReceiveBeginPlay`
  (`self.LoadData`)
  (`self.InitializeVariables`))

(event `self.ReceiveTick`
  (params (DeltaSeconds :type "Float (single-precision)")))

(event `EnhancedInput|/Game/BIN_GC/BP/PLAYER/INPUT/Movement_Action`
  (params (ActionValue :type "Vector2D Structure") (ElapsedSeconds :type "Float (double-precision)") (TriggeredSeconds :type "Float (double-precision)") (InputAction :type "InputAction Object Reference" :default "/Game/BIN_GC/BP/PLAYER/INPUT/Movement_Action.Movement_Action"))
  ; Player Movement
  (:`Triggered`
    (`self.UpdateMoveDirection` (`KismetMathLibrary.MakeVector2D` ActionValue_X ActionValue_Y))
    (`self.AddMovementInput` (`self.GetActorRightVector`) ActionValue_X)
    (`self.AddMovementInput` (`self.GetActorForwardVector`) ActionValue_Y)
    ; If Player is Moving
    (set `self.IsMoving` (`NavMovementComponent.IsMovingOnGround` (`self.CharacterMovement`))))
  (:`Completed`
    (`self.UpdateMoveDirection` (0.0 0.0))))

(event `Evt_OpenInventoryForTarget`
  (params (`InventoryUseContext ` :type "Actor Object Reference") (CloseSuccefulUse :type Boolean))
  (bind _returnvalue (`GameplayStatics.GetPlayerController` 0))
  ; Open Iventory by Target
  (`/Engine/EditorBlueprintResources/StandardMacros.IsValid` (`self.CurrentInventoryWidget`)
    (:`Is Not Valid`
      (bind _returnvalue_2 (`|CreateWidget` "/Game/BIN_GC/BP/PLAYER/UI/Menus/WBP_Inventory.WBP_Inventory_C" _returnvalue))
      (bind _output_get (set `self.CurrentInventoryWidget` _returnvalue_2))
      (`/Game/BIN_GC/BP/PLAYER/UI/Menus/WBP_Inventory.Init Inventory` _output_get self (`self.Inventory`) `InventoryUseContext ` CloseSuccefulUse)
      (`UserWidget.AddToViewport` _output_get 0)
      (`WidgetBlueprintLibrary.SetInputMode_GameAndUIEx` _returnvalue _output_get)
      (`Controller.SetIgnoreMoveInput` _returnvalue true)
      (set `PlayerController.bShowMouseCursor` true _returnvalue))))

(event `EnhancedInput|/Game/BIN_GC/BP/PLAYER/INPUT/Interact_Action`
  (params (ActionValue :type Boolean) (ElapsedSeconds :type "Float (double-precision)") (TriggeredSeconds :type "Float (double-precision)") (InputAction :type "InputAction Object Reference" :default "/Game/BIN_GC/BP/PLAYER/INPUT/Interact_Action.Interact_Action"))
  (bind _currentinteractable (`self.CurrentInteractable`))
  ; Interagir com Objetos
  (:`Completed`
    (if (and (`KismetSystemLibrary.IsValid` _currentinteractable) (`KismetSystemLibrary.DoesImplementInterface` _currentinteractable "/Game/BIN_GC/BP/GAMEPROPS/INTERACTABLES/INTERFACES/BPI_Interactable_GC.BPI_Interactable_GC_C"))
      (message `/Game/BIN_GC/BP/GAMEPROPS/INTERACTABLES/INTERFACES/BPI_Interactable_GC.Interact` _currentinteractable self))))

(event `EnhancedInput|/Game/BIN_GC/BP/PLAYER/INPUT/OpenIventory_Action`
  (params (ActionValue :type Boolean) (ElapsedSeconds :type "Float (double-precision)") (TriggeredSeconds :type "Float (double-precision)") (InputAction :type "InputAction Object Reference" :default "/Game/BIN_GC/BP/PLAYER/INPUT/OpenIventory_Action.OpenIventory_Action"))
  ; Turn Inventory
  (:`Completed`
    (`self.CurrentInventoryWidget`
      (:`then`
        (`self.Evt_CloseInventory`))
      (:`else`
        (`self.Evt_OpenInventory`)))))

(event `Evt_CloseInventory`
  (bind _returnvalue (`GameplayStatics.GetPlayerController` 0))
  (bind _currentinventorywidget (`self.CurrentInventoryWidget`))
  ; Close Inventory
  (`/Engine/EditorBlueprintResources/StandardMacros.IsValid` _currentinventorywidget
    (:`Is Valid`
      (`Widget.RemoveFromParent` _currentinventorywidget)
      (set `self.CurrentInventoryWidget` null)
      (`WidgetBlueprintLibrary.SetInputMode_GameOnly` _returnvalue)
      (set `PlayerController.bShowMouseCursor` false _returnvalue)
      (`Controller.SetIgnoreMoveInput` _returnvalue false))))

(event `Evt_OpenInventory`
  ; Open Inventory by Default
  (`self.Evt_OpenInventoryForTarget` null))

(fn `CloseMessageInteract`
  (bind _message_hud (`self.Message HUD`))
  (if (and (`KismetSystemLibrary.IsValid` _message_hud) (`self.DialogBoxOpen?`))
    (`WidgetBlueprintLibrary.SetInputMode_GameAndUIEx` (`GameplayStatics.GetPlayerController` 0) _message_hud)
    (`Widget.RemoveFromParent` _message_hud)))

(fn `GetAnimationDirectionVector`
  (returns (InputVector :type "Vector2D Structure"))
  (if (`self.IsMoving`)
    (return (`self.LastMovementVector`))
    (else
      (return (select `/Game/BIN_GC/BP/PLAYER/ENUMS/E_PlayerDirection` (`self.LastDirection`) :`NewEnumerator0` (0.0 -1.0) :`NewEnumerator1` (-1.0 0.0) :`NewEnumerator2` (1.0 0.0) :`NewEnumerator3` (0.0 1.0) :!type "Vector2D Structure")))))

(fn `InitializeVariables`
  (set `self.CurrentDirection` "NewEnumerator0"))

(fn `LoadData`)

(fn `ShowMessageInteract`
  (params (Text :type Text) (`Dialog Action` :type "/Game/BIN_GC/BP/DIALOGSYSTEM/ENUM/E_DialogueActionType Enum" :default "NewEnumerator0"))
  (bind _message_hud (`self.Message HUD`))
  (`UserWidget.AddToViewport` _message_hud 0)
  (`/Game/BIN_GC/BP/PLAYER/UI/PlayerHUD/UI_MessageContainer.SetMessageDialog` _message_hud Text `Dialog Action`)
  (`WidgetBlueprintLibrary.SetInputMode_UIOnlyEx` (`GameplayStatics.GetPlayerController` 0) _message_hud)
  (set `self.DialogBoxOpen?` true))

(fn `UpdateMoveDirection`
  (params (InputVector :type "Vector2D Structure"))
  (bind (_x _y) (`KismetMathLibrary.BreakVector2D` InputVector))
  (if (> (`KismetMathLibrary.VSize2D` InputVector) (`self.DirectionDeadZone`))
    (set `self.IsMoving` true)
    (set `self.MovementVector` InputVector)
    (set `self.LastMovementVector` (`KismetMathLibrary.Normal2D` InputVector))
    (if (> (`KismetMathLibrary.Abs` _x) (`KismetMathLibrary.Abs` _y))
      (bind _output_get (set `self.CurrentDirection` (select `bool` (> _x 0.0) :`false` "NewEnumerator0" :`true` "NewEnumerator2" :!type "/Game/BIN_GC/BP/PLAYER/ENUMS/E_PlayerDirection Enum")))
      (set `self.LastDirection` _output_get)
      (else
        (bind _output_get_2 (set `self.CurrentDirection` (select `bool` (> _y 0.0) :`false` "NewEnumerator0" :`true` "NewEnumerator3" :!type "/Game/BIN_GC/BP/PLAYER/ENUMS/E_PlayerDirection Enum")))
        (set `self.LastDirection` _output_get_2)))
    (else
      (set `self.IsMoving` false))))

(fn `UserConstructionScript`)